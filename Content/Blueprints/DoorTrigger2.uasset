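; Door trigger actor that raises a Cube component while another actor overlaps it and lowers it when the overlap ends.
; BeginPlay stores the cube's starting relative location, and the overlap events toggle a DoorUp flag.
; While Activated is true, Tick lerps the cube toward the raised or original position using delta seconds as alpha, giving an eased motion.
; Nothing in this graph sets Activated.
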(event EventTick
  (params (DeltaSeconds :type Float%20%28single-precision%29))
  (if (Variables|ActivateDoor|GetActivated)
    (if (Variables|Default|GetDoorUp)
      (Transformation|SetRelativeLocation (Variables|Default|GetCube) (Math|Vector|Lerp(Vector) (Variables|/Script/Engine.SceneComponent|GetRelativeLocation (Variables|Default|GetCube)) (+ (Variables|Default|GetOriginalPos) "0, 0,370.000000") DeltaSeconds) false false)
      (else
        (Transformation|SetRelativeLocation (Variables|Default|GetCube) (Math|Vector|Lerp(Vector) (Variables|/Script/Engine.SceneComponent|GetRelativeLocation (Variables|Default|GetCube)) (Variables|Default|GetOriginalPos) DeltaSeconds) false false)))))

(event EventBeginPlay
  (Variables|Default|SetOriginalPos (Variables|/Script/Engine.SceneComponent|GetRelativeLocation (Variables|Default|GetCube))))

(event Collision|EventActorBeginOverlap
  (params (OtherActor :type Actor%20Object%20Reference))
  (Variables|Default|SetDoorUp true))

(event Collision|EventActorEndOverlap
  (params (OtherActor :type Actor%20Object%20Reference))
  (Variables|Default|SetDoorUp false))

(fn ConstructionScript)