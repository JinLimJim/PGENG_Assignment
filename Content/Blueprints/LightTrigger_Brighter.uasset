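; LightTrigger_Brighter is an overlap-triggered actor that brightens its point light while overlapped and fades it out afterward.
; BeginPlay picks the intensity limit from a three-way PPQuality comparison, though PPQuality is hardcoded just beforehand, so only the highest limit applies.
; Overlap events toggle a flag that Tick reads to ease intensity toward that limit or zero using delta-time-scaled Lerps, rising faster than it falls.
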(event EventBeginPlay)

(event EventActorBeginOverlap
  (params (OtherActor :type Actor%20Object%20Reference))
  (Variables|Default|SetIncreaseIntensity true))

(event EventTick
  (params (DeltaSeconds :type Float%20%28single-precision%29)))

(event Collision|EventActorEndOverlap
  (params (OtherActor :type Actor%20Object%20Reference))
  (Variables|Default|SetIncreaseIntensity false))

(event EventTick
  (params (DeltaSeconds :type Float%20%28single-precision%29))
  (if (Variables|Default|GetIncreaseIntensity)
    (bind _output_get (Variables|Default|SetLightIntensity (Math|Float|Lerp (stale _output_get) (Variables|Default|GetIntensityLimit) (* DeltaSeconds 1.5))))
    (else
      (bind _output_get_2 (Variables|Default|SetLightIntensity (Math|Float|Lerp (stale _output_get_2) 0.0 DeltaSeconds)))))
  (Rendering|Components|Light|SetIntensity (Variables|Default|GetPointLight) (Variables|Default|GetLightIntensity)))

(event EventBeginPlay
  (bind _output_get (Variables|Default|SetPPQuality 2))
  (Math|Integer|CompareInt _output_get 1
    (:>
      (Variables|Default|SetIntensityLimit 8e+03))
    (:==
      (Variables|Default|SetIntensityLimit 1e+03))
    (:<
      (Variables|Default|SetIntensityLimit 4e+03))))

(fn ConstructionScript)