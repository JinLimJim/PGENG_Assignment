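; Trigger actor that fades its point light up while an actor overlaps it and back down to dark when the overlap ends.
; On BeginPlay it reads the first-person camera's post-process Quality to pick the peak intensity, using a much dimmer limit above the threshold.
; Tick lerps intensity toward that peak or zero by a delta-time alpha, easing in faster than out.
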(event EventBeginPlay)

(event EventActorBeginOverlap
  (params (OtherActor :type Actor%20Object%20Reference))
  (Variables|Default|SetIncreaseIntensity true))

(event EventTick
  (params (DeltaSeconds :type Float%20%28single-precision%29)))

(event Collision|EventActorEndOverlap
  (params (OtherActor :type Actor%20Object%20Reference))
  (Variables|Default|SetIncreaseIntensity false))

(event EventTick
  (params (DeltaSeconds :type Float%20%28single-precision%29))
  (if (Variables|Default|GetIncreaseIntensity)
    (bind _output_get (Variables|Default|SetLightIntensity (Math|Float|Lerp (stale _output_get) (Variables|Default|GetIntensityLimit) (* DeltaSeconds 1.5))))
    (else
      (bind _output_get_2 (Variables|Default|SetLightIntensity (Math|Float|Lerp (stale _output_get_2) 0.0 DeltaSeconds)))))
  (Rendering|Components|Light|SetIntensity (Variables|Default|GetPointLight) (Variables|Default|GetLightIntensity)))

(event EventBeginPlay
  (bind _outactors (Actor|GetAllActorsOfClass "/Game/FirstPersonCPP/Blueprints/FirstPersonCharacter.FirstPersonCharacter_C"))
  (for _array_element _outactors
    (bind _output_get (Variables|Default|SetPPQuality (Utilities|Struct|BreakPostProcessSettings (Variables|/Script/Engine.CameraComponent|GetPostProcessSettings (Variables|/Script/PGENG_Assignment.PGENG_AssignmentCharacter|GetFirstPersonCameraComponent _array_element)))))
    (Math|Float|CompareFloat _output_get 5e+01
      (:>
        (Variables|Default|SetIntensityLimit 5e+02))
      (:==
        (Variables|Default|SetIntensityLimit 1e+04))
      (:<
        (Variables|Default|SetIntensityLimit 1e+04)))))

(fn ConstructionScript)