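; Floating sphere Blueprint that swaps its glow material to a chosen red, blue, green or white.
; Entering the box trigger plays CueSwitch and applies the material when ReplaceMaterial is set; ChangeOnRunTime reapplies it every Tick.
; Tick also bobs the sphere by lerping between its start position and 100 units above, though the upper turnaround test compares against a fixed (0,0,100).
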(event OnComponentBeginOverlap(Boxcollision)
  (params (OtherActor :type Actor%20Object%20Reference) (OtherComp :type Primitive%20Component%20Object%20Reference) (OtherBodyIndex :type Integer) (bFromSweep :type Boolean) (SweepResult :type Hit%20Result%20Structure%20%28by%20ref%29))
  ;[1 1 1] Trigger
  (if (Variables|ColorToChange|GetReplaceMaterial)
    (Audio|Components|Audio|Play (Variables|Default|GetCueSwitch) 0.0)
    ;[1 1 1] Check and set
    (if (Utilities|Enum|Equal(Enum) (Variables|ColorToChange|GetColorToChangeTo) (Variables|ColorToChange|GetRed))
      (Variables|Default|SettheMaterial "/Game/Materials/GlowMatRed.GlowMatRed")
      (Rendering|Material|SetMaterial (Variables|Default|GetShape_Sphere) 0 (Variables|Default|GettheMaterial) :!label _label)
      (elif (Utilities|Enum|Equal(Enum) (Variables|ColorToChange|GetColorToChangeTo) (Variables|ColorToChange|GetBlue))
        (Variables|Default|SettheMaterial "/Game/Materials/GlowMatBlue.GlowMatBlue")
        (goto _label)
        (elif (Utilities|Enum|Equal(Enum) (Variables|ColorToChange|GetColorToChangeTo) (Variables|ColorToChange|GetGreen))
          (Variables|Default|SettheMaterial "/Game/Materials/GlowMatGreen.GlowMatGreen")
          (goto _label)
          (elif (Utilities|Enum|Equal(Enum) (Variables|ColorToChange|GetColorToChangeTo) (Variables|ColorToChange|GetWhite))
            (Variables|Default|SettheMaterial "/Game/Materials/GlowMatWhite.GlowMatWhite")
            (goto _label)))))))

(event EventBeginPlay
  ;[1 1 1] Ball Floating
  (Variables|Default|SetOriginalPos (Variables|/Script/Engine.SceneComponent|GetRelativeLocation (Variables|Default|GetShape_Sphere))))

(event EventTick
  (params (DeltaSeconds :type Float%20%28single-precision%29))
  (bind _shape_sphere (Variables|Default|GetShape_Sphere))
  ;[1 1 1] Ball Floating
  (if (Variables|Default|GetMoveUp)
    (Variables|Default|SetMoveUp (Math|Vector|NotEqual(Vector) (Variables|/Script/Engine.SceneComponent|GetRelativeLocation (Variables|Default|GetShape_Sphere)) "0, 0,100.000000" 1e+01))
    (Transformation|SetRelativeLocation _shape_sphere (Math|Vector|Lerp(Vector) (Variables|/Script/Engine.SceneComponent|GetRelativeLocation _shape_sphere) (+ (Variables|Default|GetOriginalPos) "0, 0,100.000000") DeltaSeconds) false false)
    (else
      (Variables|Default|SetMoveUp (Math|Vector|Equal(Vector) (Variables|/Script/Engine.SceneComponent|GetRelativeLocation (Variables|Default|GetShape_Sphere)) (Variables|Default|GetOriginalPos) 1e+01))
      (Transformation|SetRelativeLocation _shape_sphere (Math|Vector|Lerp(Vector) (Variables|/Script/Engine.SceneComponent|GetRelativeLocation _shape_sphere) (Variables|Default|GetOriginalPos) DeltaSeconds) false false)))
  ;[1 1 1] Trigger
  (if (Variables|Default|GetChangeOnRunTime)
    ;[1 1 1] Check and set
    (if (Utilities|Enum|Equal(Enum) (Variables|ColorToChange|GetColorToChangeTo) (Variables|ColorToChange|GetRed))
      (Variables|Default|SettheMaterial "/Game/Materials/GlowMatRed.GlowMatRed")
      (Rendering|Material|SetMaterial (Variables|Default|GetShape_Sphere) 0 (Variables|Default|GettheMaterial) :!label _label)
      (elif (Utilities|Enum|Equal(Enum) (Variables|ColorToChange|GetColorToChangeTo) (Variables|ColorToChange|GetBlue))
        (Variables|Default|SettheMaterial "/Game/Materials/GlowMatBlue.GlowMatBlue")
        (goto _label)
        (elif (Utilities|Enum|Equal(Enum) (Variables|ColorToChange|GetColorToChangeTo) (Variables|ColorToChange|GetGreen))
          (Variables|Default|SettheMaterial "/Game/Materials/GlowMatGreen.GlowMatGreen")
          (goto _label)
          (elif (Utilities|Enum|Equal(Enum) (Variables|ColorToChange|GetColorToChangeTo) (Variables|ColorToChange|GetWhite))
            (Variables|Default|SettheMaterial "/Game/Materials/GlowMatWhite.GlowMatWhite")
            (goto _label)))))))

(fn ConstructionScript)